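; BP_Focus is a butterfly-swarm focus point that reacts to being targeted and drives a linked effect selected by EFocus.
; Targeted runs a timeline pulling randomly colored butterflies to the center, swaps in one big butterfly and notifies the targeting actor; Untargeted reverses this.
; FocusEvent, not called within this Blueprint, either toggles which of two meshes sits at RandomTransform, plays an animation, or toggles an actor between two positions.
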(event `self.ReceiveBeginPlay`
  (bind _mesh_02 (`self.Mesh_02`))
  (bind _returnvalue_location (`KismetMathLibrary.BreakTransform` (`self.GetTransform` (`self.MoveableActor`))))
  ;[1 1 1] Array with Butterfly
  (bind _output_get (set `self.ArrayButterfly` (`|MakeArray` (`self.Butterfly01`) (`self.Butterfly02`) (`self.Butterfly03`) (`self.Butterfly04`) (`self.ButterflySmal01`) (`self.ButterflySmal02`) (`self.ButterflySmal03`))))
  (for _array_element _output_get
    ;[1 1 1] Random Material
    (`PrimitiveComponent.SetMaterial` _array_element 0 (`KismetArrayLibrary.Array_Random` (`self.ArrayMaterial`)))
    ;[1 1 1] Array Location Butterfly
    (`KismetArrayLibrary.Array_Add` (`self.ArrayLocation`) (`SceneComponent.RelativeLocation` _array_element))
    (switch `/Game/00_Christin/01_Focus/E_FocusTyp` (`self.E_Focus`)
      (:`NewEnumerator0`
        ;[1 1 1] Transfoms der Teleport Objects
        (set `self.Mesh_01_Transform` (`self.GetTransform` (`self.Mesh_01`)))
        (set `self.Mesh_02_Transform` (`self.GetTransform` _mesh_02))
        (`KismetSystemLibrary.Delay` 0.2)
        (`self.K2_SetActorTransform` _mesh_02 (`self.RandomTransform`) false true))
      (:`NewEnumerator2`
        (set `self.Position` _returnvalue_location)))))

(event `/Game/00_Christin/01_Focus/IF_Focus.Targeted`
  (params (ActorID :type "Actor Object Reference"))
  (set `self.CurrentActor` ActorID)
  (`/Engine/EditorBlueprintResources/StandardMacros.DoOnce` false :!label _label
    (:`Completed`
      (set `self.IsTargeted` true)
      (bind (_direction _length) (`Timeline|Timeline` :!label _label_2)
        (:`Update`
          ;[1 1 1] Move to Center an Backj
          (for (_array_element _array_index) (`self.ArrayButterfly`)
            (`SceneComponent.K2_SetRelativeLocation` _array_element (`KismetMathLibrary.VLerp` (`|GetArrayItem` (`self.ArrayLocation`) _array_index) (0.0 0.0 0.0) _length) true false)))
        (:`Finished`
          (switch `ETimelineDirection` _direction
            (:`Forward`
              (`self.TargetedSwitch`)
              (message `/Game/02_Character/01_Eir/IF_Character.SetOverlapBeginn` (`self.CurrentActor`)))
            (:`Backward`
              (goto _label :!via `Reset`))))))))

(event `/Game/00_Christin/01_Focus/IF_Focus.Untargeted`
  (message `/Game/02_Character/01_Eir/IF_Character.SetOverlapEnd` (`self.CurrentActor`))
  (set `self.CurrentActor` null)
  (set `self.IsTargeted` false)
  (`self.TargetedSwitch`)
  (goto _label_2 :!via `Reverse`))

(event `TargetedSwitch`
  (if (`self.IsTargeted`)
    (for _array_element (`self.ArrayButterfly`)
      (`SceneComponent.SetHiddenInGame` _array_element true false))
    (`KismetSystemLibrary.PrintString` "Niagara")
    (`KismetSystemLibrary.Delay` 0.2)
    (`SceneComponent.SetHiddenInGame` (`self.BigButterfly`) false false)
    (else
      (`SceneComponent.SetHiddenInGame` (`self.BigButterfly`) true false)
      (for _array_element_2 (`self.ArrayButterfly`)
        (`SceneComponent.SetHiddenInGame` _array_element_2 false false)))))

(event `/Game/00_Christin/01_Focus/IF_Focus.FocusEvent`
  (bind _moveableactor (`self.MoveableActor`))
  (switch `/Game/00_Christin/01_Focus/E_FocusTyp` (`self.E_Focus`)
    (:`NewEnumerator0`
      (`/Engine/EditorBlueprintResources/StandardMacros.FlipFlop`
        (:`A`
          (`self.K2_SetActorTransform` (`self.Mesh_02`) (`self.Mesh_02_Transform`) false true)
          (`self.K2_SetActorTransform` (`self.Mesh_01`) (`self.RandomTransform`) false true))
        (:`B`
          (`self.K2_SetActorTransform` (`self.Mesh_02`) (`self.RandomTransform`) false true)
          (`self.K2_SetActorTransform` (`self.Mesh_01`) (`self.Mesh_01_Transform`) false true))))
    (:`NewEnumerator1`
      (`SkeletalMeshComponent.PlayAnimation` (`SkeletalMeshActor.SkeletalMeshComponent` (`self.Anim_Actor`)) (`self.Animation`) (`self.Looping`)))
    (:`NewEnumerator2`
      (`/Engine/EditorBlueprintResources/StandardMacros.FlipFlop`
        (:`A`
          (`self.K2_SetActorLocation` _moveableactor (`self.TargetPosition`) false false))
        (:`B`
          (`self.K2_SetActorLocation` _moveableactor (`self.Position`) false false))))))

(fn `UserConstructionScript`)
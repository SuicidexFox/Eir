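; BP_AreaManager runs a combat area, switching combat state and music as the "Eir"-tagged actor enters or leaves its NavigateMesh volumes.
; Overlap events bound at BeginPlay drive two cross-resetting DoOnce gates and a delayed Back flag, messaging that actor and GameMode_Eir.
; Defeated removes entries from the AI list; once empty, it destroys the volumes and sends FocusTriggerMessage to ActorsToReact inside that loop.
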(event `self.ReceiveBeginPlay`
  (bind _asgame_mode_eir (cast `/Game/00_Christin/GameMode_Eir` (`GameplayStatics.GetGameMode`)))
  (set `self.Game Mode Eir` _asgame_mode_eir)
  (for _array_element (`self.NavigateMesh`)
    (add `self.OnActorBeginOverlap` _array_element (`|CreateDelegate` :!event `OnActorBeginOverlap_Event`))
    (add `self.OnActorEndOverlap` _array_element (`|CreateDelegate` :!event `OnActorEndOverlap_Event`))))

(event `OnActorBeginOverlap_Event` :!signature `self.OnActorBeginOverlap`
  (params (OverlappedActor :type "Actor Object Reference") (OtherActor :type "Actor Object Reference"))
  ;[0.2604 0.2604 0.2604] Overlap
  (bind _output_get (set `self.CurrentActor` OtherActor))
  (if (and (`self.ActorHasTag` _output_get "Eir") (not (`self.Back`)))
    (`|ExecutionSequence`
      (:`then_0`
        (`/Engine/EditorBlueprintResources/StandardMacros.DoOnce` false :!label _label
          (:`Completed`
            (message `/Game/00_Christin/Combat/IF_AIEnemy.CallCombat` (`self.CurrentActor`))
            (message `/Game/00_Christin/IF_GameMode.SettingsMusic` (`self.Game Mode Eir`) true)
            (`KismetSystemLibrary.Delay` 1.0)
            (set `self.Back` true))))
      (:`then_1`
        (goto _label_2 :!via `Reset`)))))

(event `OnActorEndOverlap_Event` :!signature `self.OnActorEndOverlap`
  (params (OverlappedActor :type "Actor Object Reference") (OtherActor :type "Actor Object Reference"))
  ;[0.2604 0.2604 0.2604] Overlap
  (bind _output_get (set `self.CurrentActor` OtherActor))
  (if (and (`self.ActorHasTag` _output_get "Eir") (`self.Back`))
    (`|ExecutionSequence`
      (:`then_0`
        (`/Engine/EditorBlueprintResources/StandardMacros.DoOnce` false :!label _label_2
          (:`Completed`
            (message `/Game/00_Christin/Combat/IF_AIEnemy.CallCombat` (`self.CurrentActor`))
            (message `/Game/00_Christin/IF_GameMode.SettingsMusic` (`self.Game Mode Eir`) false)
            (`KismetSystemLibrary.Delay` 1.0)
            (set `self.Back` false))))
      (:`then_1`
        (goto _label :!via `Reset`)))))

(event `Defeated`
  (params (TargetArray :type "Pawn Object Reference (by ref)"))
  (`KismetArrayLibrary.Array_RemoveItem` (`self.AI`) TargetArray)
  (if (`KismetArrayLibrary.Array_IsEmpty` (`self.AI`))
    (for _array_element (`self.NavigateMesh`)
      (`self.K2_DestroyActor` _array_element)
      (for _array_element_2 (`self.ActorsToReact`)
        (message `/Game/00_Christin/Focus/IF_FocusObject.FocusTrigger` _array_element_2)))))

(fn `UserConstructionScript`)
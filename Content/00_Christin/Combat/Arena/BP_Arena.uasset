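; BP_Arena is a combat arena actor that stages the fight intro for BP_Eir and tracks its presence in the FightBox.
; BeginnSequence disables Eir's movement, calls PlayMontage, then plays the LS_Valküre level sequence and makes FightBox visible, query-only and blocking WorldStatic.
; FightBox overlaps store or clear the Eir reference, with exit also resetting IsDistance.
; The logic to restore movement and open MainMap is unconnected.
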(event `BeginnSequence`
  (params (Target :type "Actor Object Reference"))
  (bind _fightbox (`self.FightBox`))
  (bind _asbp_eir (cast `/Game/00_Christin/Character/Eir/BP_Eir` Target))
  (bind _output_get (set `self.As BP Eir` _asbp_eir))
  (set `/Game/00_Christin/Character/Eir/BP_Eir.IsMovement` false _output_get)
  (`|PlayMontage` null
    (:`then`
      _)
    (:`OnInterrupted`
      _))
  (bind (_outactor _returnvalue) (`LevelSequencePlayer.CreateLevelSequencePlayer` "/Game/00_Christin/LevelSequence/LS_Valküre.LS_Valküre"))
  (`MovieSceneSequencePlayer.Play` _returnvalue)
  (`PrimitiveComponent.SetCollisionEnabled` _fightbox "QueryOnly")
  (`PrimitiveComponent.SetCollisionResponseToChannel` _fightbox "ECC_WorldStatic" "ECR_Block")
  (`SceneComponent.SetHiddenInGame` (`self.FightBox`) false false))

(event `self.FightBox.OnComponentBeginOverlap`
  (params (OverlappedComponent :type "PrimitiveComponent Object Reference") (OtherActor :type "Actor Object Reference") (OtherComp :type "PrimitiveComponent Object Reference") (OtherBodyIndex :type Integer) (bFromSweep :type Boolean) (SweepResult :type "HitResult Structure (by ref)"))
  (bind _asbp_eir (cast `/Game/00_Christin/Character/Eir/BP_Eir` OtherActor))
  (set `self.BP Eir` _asbp_eir))

(event `self.FightBox.OnComponentEndOverlap`
  (params (OverlappedComponent :type "PrimitiveComponent Object Reference") (OtherActor :type "Actor Object Reference") (OtherComp :type "PrimitiveComponent Object Reference") (OtherBodyIndex :type Integer))
  (cast `/Game/00_Christin/Character/Eir/BP_Eir` OtherActor)
  (set `self.BP Eir` null)
  (set `self.IsDistance` false))

(fn `UserConstructionScript`)
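; AI-controlled Draugr melee enemy with chase, attack, hit reaction and death behavior, plus getters and setters for range, movement speed, type and chase state.
; BeginPlay retries the game mode cast each tick, then notifies the AI controller and binds overlaps on DamageZone-tagged components.
; Random attack montages open an ACCombat damage window, damaging the player's HurtZone once per swing.
; Dying plays a montage while a timeline drives an opacity-mask fade.
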(event `self.ReceiveBeginPlay`
  (bind _asgame_mode_eir (cast `/Game/00_Christin/GameMode_Eir` (`GameplayStatics.GetGameMode`) :!label _label)
    (:`then`
      (set `self.GameMode` _asgame_mode_eir)
      (message `/Game/00_Christin/Combat/AI_BehaviorTree/IF_AIController.ContollerBlackboard` (`AIBlueprintHelperLibrary.GetAIController` null))
      (for _array_element (`self.GetComponentsByTag` "/Script/Engine.PrimitiveComponent" "DamageZone")
        (add `PrimitiveComponent.OnComponentBeginOverlap` _array_element (`|CreateDelegate` :!event `OnComponentBeginOverlap_Event`))))
    (:`CastFailed`
      (`KismetSystemLibrary.DelayUntilNextTick`)
      (goto _label))))

(event `/Game/00_Christin/Combat/IF_AIEnemy.AggroAnimEvent`)

(event `OnComponentBeginOverlap_Event`
  (params (OverlappedComponent :type "PrimitiveComponent Object Reference") (OtherActor :type "Actor Object Reference") (OtherComp :type "PrimitiveComponent Object Reference") (OtherBodyIndex :type Integer) (bFromSweep :type Boolean) (SweepResult :type "HitResult Structure (by ref)"))
  (bind _asbp_eir (cast `/Game/00_Christin/Eir/BP_Eir` OtherActor))
  (set `self.Player` _asbp_eir)
  (if (and (`ActorComponent.ComponentHasTag` OtherComp "HurtZone") (`/Game/00_Christin/Combat/AC_CombatValues.DamageWindow` (`self.AC_Combat`)))
    (`/Engine/EditorBlueprintResources/StandardMacros.DoOnce` false :!label _label
      (:`Completed`
        (message `/Game/00_Christin/Combat/IF_AIEnemy.Hit` OtherActor (`/Game/00_Christin/Combat/AC_CombatValues.Damage` (`self.AC_Combat`)))))))

(event `/Game/00_Christin/Combat/IF_AIEnemy.Hit`
  (params (Damage :type "Float (double-precision)"))
  (bind _ac_combat (`self.AC_Combat`))
  (set `/Game/00_Christin/Combat/AC_CombatValues.Health` (- (`/Game/00_Christin/Combat/AC_CombatValues.Health` _ac_combat) Damage) _ac_combat)
  (set `MovementComponent.Velocity` (0.0 0.0 0.0) (`self.CharacterMovement`))
  (`self.PlayAnimMontage` "/Game/02_Character/Draugr/Animations/Combat/AM_Draugr_Damage.AM_Draugr_Damage" 1.2))

(event `ResetOverlapDamageEvent`
  (goto _label :!via `Reset`))

(event `Chase`
  (`|PlayMontage` (`self.Mesh`) "/Game/02_Character/Draugr/Animations/Combat/AM_Draugr_Targeted.AM_Draugr_Targeted"
    (:`OnCompleted`
      _)
    (:`OnInterrupted`
      _))
  (`self.On Chase End`)
  (set `self.FinishChase` true))

(event `Attack`
  (bind _mesh (`self.Mesh`))
  (bind _ac_combat (`self.AC_Combat`))
  (if (`KismetMathLibrary.RandomBool`)
    (`|PlayMontage` _mesh "/Game/02_Character/Draugr/Animations/Combat/AM_Draugr_Attack01.AM_Draugr_Attack01"
      (:`then`
        (set `/Game/00_Christin/Combat/AC_CombatValues.DamageWindow` true _ac_combat :!label _label_2))
      (:`OnCompleted`
        (`self.On Attack End` :!label _label_3)
        (set `/Game/00_Christin/Combat/AC_CombatValues.DamageWindow` false _ac_combat)
        (`self.ResetOverlapDamageEvent`))
      (:`OnInterrupted`
        (goto _label_3)))
    (else
      (`|PlayMontage` _mesh "/Game/02_Character/Draugr/Animations/Combat/AM_Draugr_Attack02.AM_Draugr_Attack02"
        (:`then`
          (goto _label_2))
        (:`OnCompleted`
          (goto _label_3))
        (:`OnInterrupted`
          (goto _label_3))))))

(event `/Game/00_Christin/Combat/IF_AIEnemy.Dying`
  (params (Montage :type "AnimMontage Object Reference"))
  (`/Engine/EditorBlueprintResources/StandardMacros.DoOnce` false
    (:`Completed`
      (set `MovementComponent.Velocity` (0.0 0.0 0.0) (`self.CharacterMovement`))
      (`|PlayMontage` (`self.Mesh`) Montage
        (:`then`
          (bind (_direction _time) (`Timeline|Timeline` :!via `PlayFromStart`)
            (:`Update`
              (`MeshComponent.SetScalarParameterValueOnMaterials` (`self.Mesh`) "OpacityMask" _time))))))))

(event `/Game/00_Christin/Combat/IF_AIEnemy.Death`
  (`self.K2_DestroyActor`))

(fn `AggroCheck`
  (params (Bool :type Boolean))
  (return))

(fn `CombatValues`
  (returns (ActorComponant :type "/Game/00_Christin/Combat/AC_CombatValues Object Reference"))
  (return null))

(fn `EnemyTyp`
  (params (AITyp :type "/Game/00_Christin/Combat/Enumirator/E_AITyp Enum" :default "NewEnumerator0"))
  (returns (EnemyTyp :type Name))
  (return (select `/Game/00_Christin/Combat/Enumirator/E_AITyp` AITyp :`NewEnumerator0` "Sentry" :`NewEnumerator1` "Patrol" :!type "Name")))

(fn `GetIdealRange`
  (returns (AttackRadius :type "Float (double-precision)") (DefendRadius :type "Float (double-precision)"))
  (return (`self.Attack Radius`) (`self.Defend Radius`)))

(fn `MovementValue`
  (params (WalkSpeedTyp :type "/Game/00_Christin/Combat/Enumirator/E_AIWalkSpeed Enum" :default "NewEnumerator0"))
  (returns (Value :type "Float (double-precision)"))
  (bind _output_get (set `CharacterMovementComponent.MaxWalkSpeed` (select `/Game/00_Christin/Combat/Enumirator/E_AIWalkSpeed` WalkSpeedTyp :`NewEnumerator0` (`self.Idle`) :`NewEnumerator1` (`self.Patrol`) :`NewEnumerator2` (`self.Chase_0`)) (`self.CharacterMovement`)))
  (return _output_get))

(fn `SetChase`
  (params (SetChase :type Boolean))
  (returns (GetChase :type Boolean))
  (bind _output_get (set `self.FinishChase` SetChase))
  (return _output_get))

(fn `UserConstructionScript`)
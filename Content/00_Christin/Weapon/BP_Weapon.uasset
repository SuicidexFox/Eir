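; BP_Weapon is a weapon actor that notifies other actors when its damage zones overlap them.
; On BeginPlay it binds begin and end overlap events to every primitive component tagged DamageZone.
; A single shared DoOnce limits HitMessage calls on the overlapped actor until any end overlap resets it.
; HitMessage always passes zero, while WeaponValue separately exposes the weapon's Values.
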(event `self.ReceiveBeginPlay`
  (for _array_element (`self.GetComponentsByTag` "/Script/Engine.PrimitiveComponent" "DamageZone")
    (add `PrimitiveComponent.OnComponentBeginOverlap` _array_element (delegate `OnComponentBeginOverlap_Event`))
    (add `PrimitiveComponent.OnComponentEndOverlap` _array_element (delegate `OnComponentEndOverlap_Event`))))

(event `OnComponentBeginOverlap_Event`
  (params (OverlappedComponent :type "PrimitiveComponent Object Reference") (OtherActor :type "Actor Object Reference") (OtherComp :type "PrimitiveComponent Object Reference") (OtherBodyIndex :type Integer) (bFromSweep :type Boolean) (SweepResult :type "HitResult Structure (by ref)"))
  (`/Engine/EditorBlueprintResources/StandardMacros.DoOnce` false :!label _label
    (:`Completed`
      (message `/Game/00_Christin/Combat/IF_AIEnemy.Hit` OtherActor 0.0))))

(event `OnComponentEndOverlap_Event`
  (params (OverlappedComponent :type "PrimitiveComponent Object Reference") (OtherActor :type "Actor Object Reference") (OtherComp :type "PrimitiveComponent Object Reference") (OtherBodyIndex :type Integer))
  (goto _label :!via `Reset`))

(fn `UserConstructionScript`)

(fn `WeaponValue`
  (returns (Values :type "/Game/00_Christin/Weapon/Structure_Weapon Structure"))
  (return (`self.Values`)))
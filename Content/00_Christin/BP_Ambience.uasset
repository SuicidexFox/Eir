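; BP_Ambience is a trigger volume that signals ambience changes to the game mode when an actor tagged "Eir" enters or leaves its box.
; It caches GameMode_Eir on BeginPlay, then sends SettingsAmbienceMessage true on begin overlap and false on end overlap.
; Two DoOnce gates re-arm each other after a one-tick delay, so repeated overlap events cannot send the same message twice in a row.
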(event `self.ReceiveBeginPlay`
  (bind _asgame_mode_eir (cast `/Game/00_Christin/GameMode_Eir` (`GameplayStatics.GetGameMode`)))
  (set `self.Game Mode Eir` _asgame_mode_eir))

(event `self.Box.OnComponentBeginOverlap`
  (params (OverlappedComponent :type "PrimitiveComponent Object Reference") (OtherActor :type "Actor Object Reference") (OtherComp :type "PrimitiveComponent Object Reference") (OtherBodyIndex :type Integer) (bFromSweep :type Boolean) (SweepResult :type "HitResult Structure (by ref)"))
  (if (`self.ActorHasTag` OtherActor "Eir")
    (`/Engine/EditorBlueprintResources/StandardMacros.DoOnce` false :!label _label
      (:`Completed`
        (message `/Game/00_Christin/IF_GameMode.SettingsAmbience` (`self.Game Mode Eir`) true)
        (`KismetSystemLibrary.DelayUntilNextTick`)
        (goto _label_2 :!via `Reset`)))))

(event `self.Box.OnComponentEndOverlap`
  (params (OverlappedComponent :type "PrimitiveComponent Object Reference") (OtherActor :type "Actor Object Reference") (OtherComp :type "PrimitiveComponent Object Reference") (OtherBodyIndex :type Integer))
  (if (`self.ActorHasTag` OtherActor "Eir")
    (`/Engine/EditorBlueprintResources/StandardMacros.DoOnce` false :!label _label_2
      (:`Completed`
        (message `/Game/00_Christin/IF_GameMode.SettingsAmbience` (`self.Game Mode Eir`) false)
        (`KismetSystemLibrary.DelayUntilNextTick`)
        (goto _label :!via `Reset`)))))

(fn `UserConstructionScript`)
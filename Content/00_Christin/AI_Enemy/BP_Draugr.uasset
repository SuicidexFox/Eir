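; Draugr enemy character that chases and melee-attacks the player, Eir, with walk speed set by idle, patrol or chase state.
; Attacks play one of two random montages and open a damage window where tagged DamageZone overlaps hit Eir's HurtZone once per swing.
; Targeting and attack montages signal their end through callbacks, while hits reduce ACCombat health and halt movement.
; Death animates a material mask via timeline, then calls Eir's Equipt and destroys the actor.
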(event `self.ReceiveBeginPlay`
  (`self.SetupAttacking`)
  (bind _asgame_mode_eir (cast `/Game/00_Christin/GameMode_Eir` (`GameplayStatics.GetGameMode`)))
  (set `self.As Game Mode Eir` _asgame_mode_eir))

(event `/Game/00_Christin/Combat/IF_Combat.Hit`
  (params (Damage :type "Float (double-precision)"))
  (bind _ac_combat (`self.AC_Combat`))
  (set `/Game/00_Christin/Combat/AC_Combat.Health` (- (`/Game/00_Christin/Combat/AC_Combat.Health` _ac_combat) Damage) _ac_combat)
  (set `MovementComponent.Velocity` (0.0 0.0 0.0) (`self.CharacterMovement`))
  (`self.PlayAnimMontage` "/Game/02_Character/Draugr/Animations/Combat/AM_Draugr_Damage.AM_Draugr_Damage"))

(event `SetupAttacking`
  (for _array_element (`self.GetComponentsByTag` "/Script/Engine.PrimitiveComponent" "DamageZone")
    (add `PrimitiveComponent.OnComponentBeginOverlap` _array_element (delegate `OnComponentBeginOverlap_Event`))))

(event `OnComponentBeginOverlap_Event`
  (params (OverlappedComponent :type "PrimitiveComponent Object Reference") (OtherActor :type "Actor Object Reference") (OtherComp :type "PrimitiveComponent Object Reference") (OtherBodyIndex :type Integer) (bFromSweep :type Boolean) (SweepResult :type "HitResult Structure (by ref)"))
  (bind _asbp_eir (cast `/Game/00_Christin/Eir/BP_Eir` OtherActor))
  (set `self.Eir` _asbp_eir)
  (if (and (`ActorComponent.ComponentHasTag` OtherComp "HurtZone") (`/Game/00_Christin/Combat/AC_Combat.DamageWindow` (`self.AC_Combat`)))
    (`/Engine/EditorBlueprintResources/StandardMacros.DoOnce` false :!label _label
      (:`Completed`
        (message `/Game/00_Christin/Combat/IF_Combat.Hit` OtherActor (`/Game/00_Christin/Combat/AC_Combat.Damage` (`self.AC_Combat`)))))))

(event `ResetOverlapDamageEvent`
  (goto _label :!via `Reset`))

(event `Chase`
  (`|PlayMontage` (`self.Mesh`) "/Game/02_Character/Draugr/Animations/Combat/AM_Draugr_Targeted.AM_Draugr_Targeted"
    (:`OnCompleted`
      _)
    (:`OnInterrupted`
      _))
  (`self.On Chase End`)
  (set `self.FinishChase` true))

(event `Attack`
  (bind _mesh (`self.Mesh`))
  (bind _ac_combat (`self.AC_Combat`))
  (if (`KismetMathLibrary.RandomBool`)
    (`|PlayMontage` _mesh "/Game/02_Character/Draugr/Animations/Combat/AM_Draugr_Attack01.AM_Draugr_Attack01"
      (:`then`
        (set `/Game/00_Christin/Combat/AC_Combat.DamageWindow` true _ac_combat :!label _label_2))
      (:`OnCompleted`
        (`self.On Attack End` :!label _label_3)
        (set `/Game/00_Christin/Combat/AC_Combat.DamageWindow` false _ac_combat)
        (`self.ResetOverlapDamageEvent`))
      (:`OnInterrupted`
        (goto _label_3)))
    (else
      (`|PlayMontage` _mesh "/Game/02_Character/Draugr/Animations/Combat/AM_Draugr_Attack02.AM_Draugr_Attack02"
        (:`then`
          (goto _label_2))
        (:`OnCompleted`
          (goto _label_3))
        (:`OnInterrupted`
          (goto _label_3))))))

(event `/Game/00_Christin/Combat/IF_Combat.Dying`
  (params (Montage :type "AnimMontage Object Reference"))
  (`/Engine/EditorBlueprintResources/StandardMacros.DoOnce` false
    (:`Completed`
      (set `MovementComponent.Velocity` (0.0 0.0 0.0) (`self.CharacterMovement`))
      (`|PlayMontage` (`self.Mesh`) Montage
        (:`then`
          (bind (_direction _time) (`Timeline|T_Death`)
            (:`Update`
              (`MeshComponent.SetScalarParameterValueOnMaterials` (`self.Mesh`) "Mask" _time))))
        (:`OnCompleted`
          (`/Game/00_Christin/Eir/BP_Eir.Equipt` (`/Game/00_Christin/GameMode_Eir.Eir` (`self.As Game Mode Eir`)))
          (`self.K2_DestroyActor`))))))

(fn `CallActorComponant`
  (returns (ActorComponant :type "/Game/00_Christin/Combat/AC_Combat Object Reference"))
  (return null))

(fn `CallStates`
  (returns (States :type "/Game/00_Christin/Combat/Structur_States Structure"))
  (return))

(fn `SetMoveValue`
  (params (SpeedValue :type "/Game/00_Christin/Combat/E_MovementSpeed Enum" :default "NewEnumerator0"))
  (returns (NewSpeed :type "Float (single-precision)"))
  (bind _output_get (set `CharacterMovementComponent.MaxWalkSpeed` (select `/Game/00_Christin/Combat/E_MovementSpeed` SpeedValue :`NewEnumerator1` 120.0 :`NewEnumerator2` 300.0 :!type "Float (single-precision)") (`self.CharacterMovement`)))
  (return _output_get))

(fn `UserConstructionScript`)
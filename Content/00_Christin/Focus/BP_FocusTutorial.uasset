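; Focus-mechanic tutorial actor made of seven butterflies with random materials and animation offsets, plus one big butterfly.
; Targeting plays a timeline that gathers the butterflies at the actor's origin, crossfades masks toward the big butterfly and drives linked FocusActors' emissive; untargeting reverses it.
; Completing the timeline validates focus.
; The focus event plays audio and triggers FocusActors, then either untargets or fades out, removes the tutorial widget and destroys itself.
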(event `self.ReceiveBeginPlay`
  ;[1 1 1] Array with Butterfly
  (bind _output_get (set `self.ArrayButterfly` (`|MakeArray` (`self.Butterfly01`) (`self.Butterfly02`) (`self.Butterfly03`) (`self.Butterfly04`) (`self.ButterflySmal01`) (`self.ButterflySmal02`) (`self.ButterflySmal03`))))
  (for _array_element _output_get
    ;[1 1 1] Random Material
    (`PrimitiveComponent.SetMaterial` _array_element 0 (`KismetArrayLibrary.Array_Random` (`self.ArrayMaterial`)))
    ;[1 1 1] Array Location Butterfly
    (`KismetArrayLibrary.Array_Add` (`self.ArrayLocation`) (`SceneComponent.RelativeLocation` _array_element))
    (`MeshComponent.SetScalarParameterValueOnMaterials` (`self.BigButterfly`) "Mask" 0.0)
    (`SkeletalMeshComponent.SetPosition` _array_element (`KismetMathLibrary.RandomFloatInRange` 0.0 1.0) true)
    (bind _asgame_mode_eir (cast `/Game/00_Christin/GameMode_Eir` (`GameplayStatics.GetGameMode`)))
    (set `self.GameMode` _asgame_mode_eir)))

(event `self.FocusEvent`
  (bind _tutorial_stack (`/Game/04_UI/Player/CAW_PlayerHUD.Tutorial_Stack` (`/Game/00_Christin/Eir/BP_Eir.CAW Player` (`/Game/00_Christin/GameMode_Eir.BPEir` (`self.GameMode`)))))
  (`FMODBlueprintStatics.PlayEventAtLocation` "/Game/FMOD/Events/SFX/Eir/Focus/FocusTrigger.FocusTrigger" (`self.GetTransform`))
  (for _array_element (`self.FocusActor`)
    (message `/Game/00_Christin/Focus/IF_FocusObject.FocusTrigger` _array_element)
    (if (`self.Destroy`)
      (bind (_direction _emissive) (`Timeline|T_Destroy`)
        (:`Update`
          (`MeshComponent.SetScalarParameterValueOnMaterials` (`self.BigButterfly`) "Mask" _emissive)
          (`SceneComponent.SetVisibility` (`self.ButterflySmal03`) false false)
          (`SceneComponent.SetVisibility` (`self.ButterflySmal02`) false false)
          (`SceneComponent.SetVisibility` (`self.ButterflySmal01`) false false)
          (`SceneComponent.SetVisibility` (`self.Butterfly04`) false false)
          (`SceneComponent.SetVisibility` (`self.Butterfly03`) false false)
          (`SceneComponent.SetVisibility` (`self.Butterfly02`) false false)
          (`SceneComponent.SetVisibility` (`self.Butterfly01`) false false))
        (:`Finished`
          (`CommonActivatableWidgetContainerBase.RemoveWidget` _tutorial_stack (`CommonActivatableWidgetContainerBase.GetActiveWidget` _tutorial_stack))
          (`self.K2_DestroyActor`)))
      (else
        (message `/Game/00_Christin/Focus/IF_Focus.Untargeted` (`self.Actor ID`))))))

(event `self.Targeted`
  (params (ActorID :type "Actor Object Reference"))
  (bind _arraybutterfly (`self.ArrayButterfly`))
  (set `self.Actor ID` ActorID)
  (`/Engine/EditorBlueprintResources/StandardMacros.DoOnce` false :!label _label
    (:`Completed`
      (bind (_direction _move _maskoff _maskon _emissive) (`Timeline|Time_Targeted` :!label _label_2)
        (:`Update`
          (for _array_element (`self.FocusActor`)
            (message `/Game/00_Christin/Focus/IF_FocusObject.ObejectEmissive` _array_element _emissive)
            (for (_array_element_2 _array_index) (`self.ArrayButterfly`)
              (`SceneComponent.K2_SetRelativeLocation` _array_element_2 (`KismetMathLibrary.VLerp` (`|GetArrayItem` (`self.ArrayLocation`) _array_index) (0.0 0.0 0.0) _move) true false) ; MoveButterfly
              (for (_ _array_index_2) _arraybutterfly
                (`MeshComponent.SetScalarParameterValueOnMaterials` (`|GetArrayItem` _arraybutterfly _array_index_2) "Mask" (`KismetMathLibrary.Lerp` 0.0 1.0 _maskoff)) ; MateriallSmalButterfly
                (`MeshComponent.SetScalarParameterValueOnMaterials` (`self.BigButterfly`) "Mask" (`KismetMathLibrary.Lerp` 0.0 1.0 _maskon)) ; MaterialBigButterfly
              ))))
        (:`Finished`
          (switch `ETimelineDirection` _direction
            (:`Forward`
              (set `self.ValideFocusEvent` true))
            (:`Backward`
              (goto _label :!via `Reset`))))))))

(event `self.Untargeted`
  (set `self.ValideFocusEvent` false)
  (goto _label_2 :!via `Reverse`))

(fn `UserConstructionScript`)

(fn `validFocusEvent`
  (returns (valideFocusEvent :type Boolean))
  (return (`self.ValideFocusEvent`)))
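; BP_FocusObject is an actor that changes location when its focus trigger fires, acting as either a Teleport or Moveable object by type.
; Teleport jumps to the target or the BeginPlay-cached location depending on IsA, which this graph never changes.
; Moveable makes one fixed-delta TInterpTo step from the cached start toward the target per trigger, applying location only.
; SetObjectTyp, despite its name, only returns the type.
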(event `self.ReceiveBeginPlay`
  (set `self.ActorTransform` (`self.GetTransform`)))

(event `/Game/00_Christin/Focus/IF_FocusObject.FocusTrigger`
  (switch `/Game/00_Christin/Focus/E_FocusObjectTyp` (`self.ObjectTyp`)
    (:`NewEnumerator0`
      (`self.Switch`))
    (:`NewEnumerator2`
      (`self.Moveable`))))

(event `Moveable`
  (`self.K2_SetActorLocation` (.location (`KismetMathLibrary.TInterpTo` (`self.ActorTransform`) (`self.TargetTransform`) 0.2 (`self.Speed`)))))

(event `Switch`
  (if (`self.IsA`)
    (`self.K2_SetActorLocation` (.location (`self.TargetTransform`)) false true)
    (else
      (`self.K2_SetActorLocation` (.location (`self.ActorTransform`)) false true))))

(fn `SetObjectTyp`
  (returns (Typ :type "/Game/00_Christin/Focus/E_FocusObjectTyp Enum"))
  (return (`self.ObjectTyp`)))

(fn `UserConstructionScript`)
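; BP_InteractObject is an interactable prop whose type makes it either switch between solid mesh and Niagara-style static mesh, or play an animation.
; FocusTrigger, called externally or by a one-time box overlap with an "Eir"-tagged actor, runs the matching behavior.
; Switching drives a "Mask" material parameter through a reversible timeline, toggling visibility and collision.
; Animation plays a clip, optionally followed by a loop; a helper sets material emissive.
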(event `self.ReceiveBeginPlay`
  (switch `/Game/00_Christin/Focus/E_FocusObjectTyp` (`self.ObjectTyp`)
    (:`NewEnumerator0`
      (if (`self.Niagara`)
        (`SceneComponent.SetVisibility` (`self.Mesh`) false false)
        (`SceneComponent.SetVisibility` (`self.NS_StaticMesh`) true false)
        (`SceneComponent.SetVisibility` (`self.SkeletalMesh`) false true)
        (`PrimitiveComponent.SetCollisionEnabled` (`self.Mesh`) "NoCollision")
        (else
          (`SceneComponent.SetVisibility` (`self.SkeletalMesh`) false true)
          (`SceneComponent.SetVisibility` (`self.Mesh`) true false)
          (`SceneComponent.SetVisibility` (`self.NS_StaticMesh`) false false))))
    (:`NewEnumerator1`
      (`SceneComponent.SetVisibility` (`self.Mesh`) false true)
      (`SkeletalMeshComponent.PlayAnimation` (`self.SkeletalMesh`) (`self.StartAnimation`) true))))

(event `/Game/00_Christin/Focus/IF_FocusObject.FocusTrigger`
  (switch `/Game/00_Christin/Focus/E_FocusObjectTyp` (`self.ObjectTyp`)
    (:`NewEnumerator0`
      (`self.Switch`))
    (:`NewEnumerator1`
      (`self.Animation`))))

(event `Switch`
  (bind _mesh (`self.Mesh`))
  (if (not (`self.Niagara`))
    (set `self.Niagara` true)
    (bind (_direction _material) (`Timeline|TL_Material` :!label _label)
      (:`Update`
        (`MeshComponent.SetScalarParameterValueOnMaterials` (`self.Mesh`) "Mask" _material)
        (`PrimitiveComponent.SetCollisionEnabled` (`self.Mesh`) "NoCollision"))
      (:`Finished`
        (switch `ETimelineDirection` _direction
          (:`Forward`
            (`SceneComponent.SetVisibility` (`self.Mesh`) false false)
            (`SceneComponent.SetVisibility` (`self.NS_StaticMesh`) true false))
          (:`Backward`
            (`PrimitiveComponent.SetCollisionEnabled` _mesh "QueryOnly")
            (`PrimitiveComponent.SetCollisionResponseToChannel` _mesh "ECC_WorldStatic" "ECR_Block")))))
    (else
      (set `self.Niagara` false)
      (`SceneComponent.SetVisibility` (`self.Mesh`) true false)
      (`SceneComponent.SetVisibility` (`self.NS_StaticMesh`) false false)
      (goto _label :!via `Reverse`))))

(event `Animation`
  (bind _skeletalmesh (`self.SkeletalMesh`))
  (bind _newanimation (`self.NewAnimation`))
  (`SkeletalMeshComponent.PlayAnimation` _skeletalmesh _newanimation false)
  (if (`self.Looping`)
    (`KismetSystemLibrary.Delay` (`AnimationAsset.GetPlayLength` _newanimation))
    (`SkeletalMeshComponent.PlayAnimation` _skeletalmesh (`self.LoopingAnimation`) true)))

(event `self.Box.OnComponentBeginOverlap`
  (params (OverlappedComponent :type "PrimitiveComponent Object Reference") (OtherActor :type "Actor Object Reference") (OtherComp :type "PrimitiveComponent Object Reference") (OtherBodyIndex :type Integer) (bFromSweep :type Boolean) (SweepResult :type "HitResult Structure (by ref)"))
  (if (and (`self.Overlap`) (`self.ActorHasTag` OtherActor "Eir"))
    (`/Engine/EditorBlueprintResources/StandardMacros.DoOnce` false
      (:`Completed`
        (`/Game/00_Christin/Focus/IF_FocusObject.FocusTrigger`)))))

(fn `ObejectEmissive`
  (params (Emissive :type "Float (double-precision)"))
  (`MeshComponent.SetScalarParameterValueOnMaterials` (`self.Mesh`) "Emissive" Emissive) ; MaterialBigButterfly
  (return))

(fn `SetObjectTyp`
  (returns (Typ :type "/Game/00_Christin/Focus/E_FocusObjectTyp Enum"))
  (return (`self.ObjectTyp`)))

(fn `UserConstructionScript`)
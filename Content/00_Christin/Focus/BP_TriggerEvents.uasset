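; BP_TriggerEvents is a one-shot trigger actor that fires optional player, music and ambience changes when the Eir player character overlaps it.
; BeginPlay caches BP_Eir and GameMode_Eir; overlap sends CombatStates to Eir and music and ambience events to the game mode, each gated by a flag, then destroys the trigger.
; An ActorReact event calls Moveable on listed BP_FocusObjects, but the overlap chain does not invoke it.
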(event `self.ReceiveBeginPlay`
  (bind _asbp_eir (cast `/Game/00_Christin/Eir/BP_Eir` (`GameplayStatics.GetPlayerCharacter` 0)))
  (set `self.Eir` _asbp_eir)
  (bind _asgame_mode_eir (cast `/Game/00_Christin/GameMode_Eir` (`GameplayStatics.GetGameMode`)))
  (set `self.Game Mode Eir` _asgame_mode_eir))

(event `self.ReceiveActorBeginOverlap`
  (params (OtherActor :type "Actor Object Reference"))
  (if (== OtherActor (`self.Eir`))
    (`self.SetupPlayer`)
    (`self.SetupMusic`)
    (`self.SetupAmbience`)
    (`self.K2_DestroyActor`)))

(event `SetupPlayer`
  (if (`self.Player`)
    (message `/Game/00_Christin/Combat/IF_Combat.SendStates` (`self.Eir`) (`self.Combat States`))))

(event `ActorReact`
  (if (`self.Actor`)
    (for _array_element (`self.ActorToReact`)
      (bind _asbp_focus_object (cast `/Game/00_Christin/Focus/BP_FocusObject` _array_element))
      (`/Game/00_Christin/Focus/BP_FocusObject.Moveable` _asbp_focus_object))))

(event `SetupMusic`
  (if (`self.Music`)
    (`/Game/00_Christin/GameMode_Eir.SetupMusic` (`self.Game Mode Eir`) (`self.MusicEvent`))))

(event `SetupAmbience`
  (if (`self.Ambience`)
    (`/Game/00_Christin/GameMode_Eir.SetupAmbience` (`self.Game Mode Eir`) (`self.AmbienceEvent`))))

(fn `UserConstructionScript`)
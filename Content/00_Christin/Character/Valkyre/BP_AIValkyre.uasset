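; Valkyrie AI character that triggers an ending cinematic and level change when Eir reaches it.
; On Eir's first overlap with its sphere, it plays an ascendant transition animation and hands a level sequence to GameMode_Eir, whose end callback opens the main map.
; It also initializes health and exposes functions for death state, combat radii, enemy type, walk speed by movement state and the animation damage window.
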(event `self.ReceiveBeginPlay`
  (bind _asgame_mode_eir (cast `/Game/00_Christin/GameMode_Eir` (`GameplayStatics.GetGameMode`)))
  (set `self.GameMode` _asgame_mode_eir)
  (set `self.CurrentHealth` (`self.MaxHealth`)))

(event `self.Sphere.OnComponentBeginOverlap`
  (params (OverlappedComponent :type "PrimitiveComponent Object Reference") (OtherActor :type "Actor Object Reference") (OtherComp :type "PrimitiveComponent Object Reference") (OtherBodyIndex :type Integer) (bFromSweep :type Boolean) (SweepResult :type "HitResult Structure (by ref)"))
  (bind _gamemode (`self.GameMode`))
  (if (`self.ActorHasTag` OtherActor "Eir")
    (`/Engine/EditorBlueprintResources/StandardMacros.DoOnce` false
      (:`Completed`
        (`SkeletalMeshComponent.PlayAnimation` (`self.Mesh`) "/Game/00_Christin/Character/Valkyre/Animation/Combat/A_root_V_AscendantTransition.A_root_V_AscendantTransition" false)
        (`/Game/00_Christin/GameMode_Eir.Sequence` _gamemode (`self.Level Sequence`))
        (add `/Game/00_Christin/GameMode_Eir.On Sequence End` _gamemode (delegate `CustomEvent`))))))

(event `CustomEvent`
  (`GameplayStatics.OpenLevelBySoftObjectPtr` "/Game/00_Maeve/MainMap.MainMap"))

(fn `AnimEvent_DamageWindow`
  (params (DamageWindow :type Boolean :default false))
  (set `self.DamageWindow` DamageWindow)
  (return))

(fn `AskDead`
  (returns (isDead :type Boolean))
  (return (`self.IsDead`)))

(fn `EnemyTyp`
  (returns (AITyp :type "/Game/00_Christin/Combat/Enumirator/E_AITyp Enum"))
  (return (`self.Typ`)))

(fn `GetIdealRange`
  (returns (AttackRadius :type "Float (double-precision)") (DefendRadius :type "Float (double-precision)"))
  (return (`self.Attack Radius`) (`self.Defend Radius`)))

(fn `MovementValue`
  (params (WalkSpeedTyp :type "/Game/00_Christin/Combat/Enumirator/E_AIWalkSpeed Enum" :default "NewEnumerator0"))
  (returns (Value :type "Float (double-precision)"))
  (bind _output_get (set `CharacterMovementComponent.MaxWalkSpeed` (select `/Game/00_Christin/Combat/Enumirator/E_AIWalkSpeed` WalkSpeedTyp :`NewEnumerator1` (`self.Patrol`) :`NewEnumerator2` (`self.Chase`)) (`self.CharacterMovement`)))
  (return _output_get))

(fn `UserConstructionScript`)
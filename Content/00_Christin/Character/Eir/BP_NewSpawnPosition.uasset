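; BP_NewSpawnPosition is a checkpoint actor that sets a new spawn position for the Eir character.
; On the first valid overlap with a BP_Eir tagged "Eir", it copies its own transform into that character's SpawnPosition, with a DoOnce blocking later updates.
; BeginPlay caches the Eir game mode, though the graphs shown do not use that reference.
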(event `self.ReceiveBeginPlay`
  (bind _asgame_mode_eir (cast `/Game/00_Christin/GameMode_Eir` (`GameplayStatics.GetGameMode`)))
  (set `self.Game Mode Eir` _asgame_mode_eir))

(event `self.ReceiveActorBeginOverlap`
  (params (OtherActor :type "Actor Object Reference"))
  (if (`self.ActorHasTag` OtherActor "Eir")
    (bind _asbp_eir (cast `/Game/00_Christin/Character/Eir/BP_Eir` OtherActor))
    (set `self.Eir` _asbp_eir)
    (`/Engine/EditorBlueprintResources/StandardMacros.DoOnce` false
      (:`Completed`
        (set `/Game/00_Christin/Character/Eir/BP_Eir.SpawnPosition` (`self.GetTransform`) (`self.Eir`))))))

(fn `UserConstructionScript`)
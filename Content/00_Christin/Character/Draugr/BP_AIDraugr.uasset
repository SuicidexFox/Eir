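; AI-controlled Draugr enemy that fights the player Eir, with a health bar and montages for patrol, detection, attacks, damage, stagger and death.
; Dispatchers report montage endings, while interface-style functions expose speed, ranges, type and death state.
; Anim-driven damage windows gate left and right hitboxes, with DoOnce limiting repeat hits.
; A linked Area toggles combat state and music; death destroys it and any Arena, then dissolves the mesh through a material mask.
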(event `self.ReceiveBeginPlay`
  (bind _area (`self.Area`))
  (bind _asgame_mode_eir (cast `/Game/00_Christin/GameMode_Eir` (`GameplayStatics.GetGameMode`)))
  (set `self.GameMode` _asgame_mode_eir)
  (bind _aswbp_healthbar (cast `/Game/00_Christin/Character/Draugr/WBP_Healthbar` (`WidgetComponent.GetWidget` (`self.HealthBar`))))
  (set `self.WBPHealthbar` _aswbp_healthbar)
  (set `self.CurrentHealth` (`self.MaxHealth`))
  (message `/Game/00_Christin/Combat/IF_AIController.ContollerBlackboard` (`AIBlueprintHelperLibrary.GetAIController` null))
  (add `PrimitiveComponent.OnComponentBeginOverlap` (`self.DamageBoxRight`) (`|CreateDelegate` :!event `OnDamageOverlapRight`))
  (add `PrimitiveComponent.OnComponentBeginOverlap` (`self.DamageBoxLeft`) (`|CreateDelegate` :!event `OnDamageOverlampLeft`))
  (add `self.OnActorBeginOverlap` _area (`|CreateDelegate` :!event `OnActorBeginOverlap_Event`))
  (add `self.OnActorEndOverlap` _area (`|CreateDelegate` :!event `OnActorEndOverlap_Event`)))

(event `Idle Variance`
  (`|PlayMontage` (`self.Mesh`) (`KismetArrayLibrary.Array_Random` (`self.PatrolMontage`))
    (:`OnCompleted`
      _)
    (:`OnInterrupted`
      _))
  (`self.On Patrol End`))

(event `self.ReceiveTick`
  (params (DeltaSeconds :type "Float (single-precision)"))
  (set `/Game/00_Christin/Character/Draugr/WBP_Healthbar.HealPercent` (`KismetMathLibrary.MapRangeClamped` (`self.CurrentHealth`) 0.0 (`self.MaxHealth`) 0.0 1.0) (`self.WBPHealthbar`)))

(event `OnActorBeginOverlap_Event` :!signature `self.OnActorBeginOverlap`
  (params (OverlappedActor :type "Actor Object Reference") (OtherActor :type "Actor Object Reference"))
  (bind _output_get (set `self.CurrentActor` OtherActor))
  (if (and (`self.ActorHasTag` _output_get "Eir") (not (`self.Back`)))
    (`|ExecutionSequence`
      (:`then_0`
        (`/Engine/EditorBlueprintResources/StandardMacros.DoOnce` false :!label _label
          (:`Completed`
            (message `/Game/00_Christin/Combat/IF_Combat.ToggleCombateState` (`self.CurrentActor`))
            (message `/Game/00_Christin/IF_GameMode.SettingsMusic` (`self.GameMode`) true)
            (`KismetSystemLibrary.Delay` 2.0)
            (set `self.Back` true))))
      (:`then_1`
        (goto _label_2 :!via `Reset`)))))

(event `OnActorEndOverlap_Event` :!signature `self.OnActorEndOverlap`
  (params (OverlappedActor :type "Actor Object Reference") (OtherActor :type "Actor Object Reference"))
  (bind _output_get (set `self.CurrentActor` OtherActor))
  (if (and (`self.ActorHasTag` _output_get "Eir") (`self.Back`))
    (`|ExecutionSequence`
      (:`then_0`
        (`/Engine/EditorBlueprintResources/StandardMacros.DoOnce` false :!label _label_2
          (:`Completed`
            (message `/Game/00_Christin/Combat/IF_Combat.ToggleCombateState` (`self.CurrentActor`))
            (message `/Game/00_Christin/IF_GameMode.SettingsMusic` (`self.GameMode`) false)
            (`KismetSystemLibrary.Delay` 2.0)
            (set `self.Back` false))))
      (:`then_1`
        (goto _label :!via `Reset`)))))

(event `AnimEvent_DamageWindow_1_1`
  (params (Right :type Boolean)))

(event `OnDamageOverlapRight`
  (params (OverlappedComponent :type "PrimitiveComponent Object Reference") (OtherActor :type "Actor Object Reference") (OtherComp :type "PrimitiveComponent Object Reference") (OtherBodyIndex :type Integer) (bFromSweep :type Boolean) (SweepResult :type "HitResult Structure (by ref)"))
  (if (and (`ActorComponent.ComponentHasTag` OtherComp "Hurt") (`self.DamageWindow`) (`self.ActorHasTag` OtherActor "Eir"))
    (`/Engine/EditorBlueprintResources/StandardMacros.DoOnce` false :!label _label
      (:`Completed`
        (message `/Game/00_Christin/Combat/IF_Combat.TriggerDamage` OtherActor (`self.Damage`))))))

(event `/Game/00_Christin/Combat/IF_Combat.TriggerDamage`
  (params (DamageValue :type "Float (double-precision)"))
  (set `self.CurrentHealth` (- (`self.CurrentHealth`) DamageValue))
  (if (<= (`self.CurrentHealth`) 0.0)
    (set `self.IsDead` true)
    (`self.TriggerDying`)
    (else
      (`|PlayMontage` (`self.Mesh`) "/Game/00_Christin/Character/Draugr/Animations/Combat/AM_Draugr_Damage.AM_Draugr_Damage" 2.0))))

(event `/Game/00_Christin/Combat/IF_Combat.ResetDamageBox`
  (`|ExecutionSequence`
    (:`then_0`
      (goto _label :!via `Reset`))
    (:`then_1`
      (goto _label_2 :!via `Reset`))))

(event `/Game/00_Christin/Combat/IF_Combat.TriggerStunned`
  (`|PlayMontage` (`self.Mesh`) "/Game/00_Christin/Character/Draugr/Animations/Combat/AM_Draugr_Staggerd.AM_Draugr_Staggerd" 2.0))

(event `OnDamageOverlampLeft`
  (params (OverlappedComponent :type "PrimitiveComponent Object Reference") (OtherActor :type "Actor Object Reference") (OtherComp :type "PrimitiveComponent Object Reference") (OtherBodyIndex :type Integer) (bFromSweep :type Boolean) (SweepResult :type "HitResult Structure (by ref)"))
  (if (and (`ActorComponent.ComponentHasTag` OtherComp "Hurt") (`self.DamageWindow`) (`self.ActorHasTag` OtherActor "Eir"))
    (`/Engine/EditorBlueprintResources/StandardMacros.DoOnce` false :!label _label_2
      (:`Completed`
        (message `/Game/00_Christin/Combat/IF_Combat.TriggerDamage` OtherActor (`self.Damage`))))))

(event `/Game/00_Christin/Combat/IF_Combat.ResetHeal`
  (set `self.CurrentHealth` (`self.MaxHealth`))
  (`SceneComponent.SetHiddenInGame` (`self.HealthBar`) true false))

(event `/Game/00_Christin/Combat/IF_Combat.TriggerDetected`
  (`SceneComponent.SetHiddenInGame` (`self.HealthBar`) false false)
  (`|PlayMontage` (`self.Mesh`) "/Game/00_Christin/Character/Draugr/Animations/Combat/AM_Draugr_Targeted.AM_Draugr_Targeted"
    (:`OnCompleted`
      _)
    (:`OnInterrupted`
      _))
  (`self.On Detected End`))

(event `/Game/00_Christin/Combat/IF_Combat.TriggerAttack`
  (bind _mesh (`self.Mesh`))
  (if (`KismetMathLibrary.RandomBool`)
    (`|PlayMontage` _mesh "/Game/00_Christin/Character/Draugr/Animations/Combat/AM_Draugr_Attack01.AM_Draugr_Attack01" 2.0
      (:`OnCompleted`
        _)
      (:`OnInterrupted`
        _))
    (else
      (`|PlayMontage` _mesh "/Game/00_Christin/Character/Draugr/Animations/Combat/AM_Draugr_Attack02.AM_Draugr_Attack02" 1.5
        (:`OnCompleted`
          _)
        (:`OnInterrupted`
          _))))
  (`self.On Attack End`)
  (`self.ResetDamageBox`))

(event `/Game/00_Christin/Combat/IF_Combat.TriggerDying`
  (`/Engine/EditorBlueprintResources/StandardMacros.DoOnce` false
    (:`Completed`
      (`|PlayMontage` (`self.Mesh`) "/Game/00_Christin/Character/Draugr/Animations/Combat/AM_Draugr_Dying.AM_Draugr_Dying"
        (:`then`
          (message `/Game/00_Christin/Focus/IF_FocusObject.FocusTrigger` (`self.ActorToReact`))
          (`self.K2_DestroyActor` (`self.Area`))
          (bind _arena (`self.Arena`)
            (:`then`
              (`self.K2_DestroyActor` _arena))
            (:`else`)))))))

(event `/Game/00_Christin/Combat/IF_Combat.AnimEvent_Dead`
  (bind (_direction _time) (`Timeline|TL_Dying` :!via `PlayFromStart`)
    (:`Update`
      (`MeshComponent.SetScalarParameterValueOnMaterials` (`self.Mesh`) "Mask" _time))
    (:`Finished`
      (if (`self.Tutorial`)
        _
        (else
          _))
      (`self.K2_DestroyActor`))))

(fn `AnimEvent_DamageWindow`
  (params (DamageWindow :type Boolean))
  (set `self.DamageWindow` DamageWindow)
  (return))

(fn `AskDead`
  (returns (isDead :type Boolean))
  (return (`self.IsDead`)))

(fn `EnemyTyp`
  (returns (AITyp :type "/Game/00_Christin/Combat/Enumirator/E_AITyp Enum"))
  (return (`self.Typ`)))

(fn `GetIdealRange`
  (returns (AttackRadius :type "Float (double-precision)") (DefendRadius :type "Float (double-precision)"))
  (return (`self.Attack Radius`) (`self.Defend Radius`)))

(fn `MovementValue`
  (params (WalkSpeedTyp :type "/Game/00_Christin/Combat/Enumirator/E_AIWalkSpeed Enum" :default "NewEnumerator0"))
  (returns (Value :type "Float (double-precision)"))
  (bind _output_get (set `CharacterMovementComponent.MaxWalkSpeed` (select `/Game/00_Christin/Combat/Enumirator/E_AIWalkSpeed` WalkSpeedTyp :`NewEnumerator1` (`self.Patrol`) :`NewEnumerator2` (`self.Chase`)) (`self.CharacterMovement`)))
  (return _output_get))

(fn `UserConstructionScript`)
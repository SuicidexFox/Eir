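; BP_Draugr is the Draugr enemy character, handling melee hit detection, damage and death.
; On BeginPlay, components tagged "DemegeZone" are unhidden and send a Hit message with ACCombat damage when overlapping similarly tagged components.
; Incoming hits reduce ACCombat health and play a damage montage only while DamageWindow is set.
; Death animates the material "Mask" parameter via timeline, then destroys the actor.
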(event `self.ReceiveBeginPlay`
  (`self.SetupAttacking`)
  (`KismetSystemLibrary.K2_SetTimer` null "Test" 1.0 true true))

(event `SetupAttacking`
  (if true
    (for _array_element (`self.GetComponentsByTag` "/Script/Engine.PrimitiveComponent" "DemegeZone")
      (add `PrimitiveComponent.OnComponentBeginOverlap` _array_element (delegate `OnComponentBeginOverlap_Event`))
      (`SceneComponent.SetHiddenInGame` _array_element false false))))

(event `OnComponentBeginOverlap_Event`
  (params (OverlappedComponent :type "PrimitiveComponent Object Reference") (OtherActor :type "Actor Object Reference") (OtherComp :type "PrimitiveComponent Object Reference") (OtherBodyIndex :type Integer) (bFromSweep :type Boolean) (SweepResult :type "HitResult Structure (by ref)"))
  (if (`ActorComponent.ComponentHasTag` OtherComp "DemegeZone")
    (message `/Game/00_Christin/Combat/IF_Combat.Hit` OtherActor (`/Game/00_Christin/Combat/AC_Combat.Damage` (`self.AC_Combat`)))))

(event `/Game/00_Christin/Combat/IF_Combat.Hit`
  (params (Damage :type "Float (double-precision)"))
  (bind _ac_combat (`self.AC_Combat`))
  (if (`/Game/00_Christin/Combat/AC_Combat.DamageWindow` _ac_combat)
    (set `/Game/00_Christin/Combat/AC_Combat.Health` (- (`/Game/00_Christin/Combat/AC_Combat.Health` _ac_combat) Damage) _ac_combat)
    (`self.PlayAnimMontage` "/Game/02_Character/Draugr/Animations/AM_Draugr_Damage.AM_Draugr_Damage")))

(event `/Game/00_Christin/Combat/IF_Combat.Death`
  (bind (_direction _time) (`Timeline|T_Death` :!via `PlayFromStart`)
    (:`Update`
      (`MeshComponent.SetScalarParameterValueOnMaterials` (`self.Mesh`) "Mask" _time))
    (:`Finished`
      (`self.K2_DestroyActor`))))

(fn `CallActorComponant`
  (returns (ActorComponant :type "/Game/00_Christin/Combat/AC_Combat Object Reference"))
  (return null))

(fn `CallStates`
  (returns (States :type "/Game/00_Christin/Combat/Structur_States Structure"))
  (return))

(fn `UpdateWalkSpeed`
  (params (NewWalkSpeed :type "Float (double-precision)"))
  (set `CharacterMovementComponent.MaxWalkSpeed` NewWalkSpeed (`self.CharacterMovement`)))

(fn `UserConstructionScript`)
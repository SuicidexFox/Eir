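; Draugr enemy AI character that fights with randomly chosen melee montages, takes hits, shows a healthbar in combat and dies.
; Tagged damage-zone primitives hit HurtZone components once per attack while the damage window is open.
; Montage endings fire end callbacks, while functions expose death state, type, ideal ranges and walk speed.
; Death animates a material mask via timeline, notifies its manager, clears any tutorial widget and destroys the actor.
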(event `self.ReceiveBeginPlay`
  (bind _asgame_mode_eir (cast `/Game/00_Christin/GameMode_Eir` (`GameplayStatics.GetGameMode`) :!label _label)
    (:`then`
      (set `self.GameMode` _asgame_mode_eir)
      (message `/Game/00_Christin/Combat/AI_BehaviorTree/IF_AIController.ContollerBlackboard` (`AIBlueprintHelperLibrary.GetAIController` null))
      (for _array_element (`self.GetComponentsByTag` "/Script/Engine.PrimitiveComponent" "DamageZone")
        (add `PrimitiveComponent.OnComponentBeginOverlap` _array_element (`|CreateDelegate` :!event `OnComponentBeginOverlap_Event`))
        (bind _aswbp_healthbar (cast `/Game/00_Christin/Draugr/WBP_Healthbar` (`WidgetComponent.GetWidget` (`self.HealthBar`))))
        (set `self.WBPHealthbar` _aswbp_healthbar)
        (set `self.CurrentHealth` (`self.MaxHealth`))))
    (:`CastFailed`
      (`KismetSystemLibrary.DelayUntilNextTick`)
      (goto _label))))

(event `Idle Variance`
  (`|PlayMontage` (`self.Mesh`) (`KismetArrayLibrary.Array_Random` (`self.IdleVariance`))
    (:`OnCompleted`
      _)
    (:`OnInterrupted`
      _))
  (`self.On Idle End`))

(event `self.ReceiveTick`
  (params (DeltaSeconds :type "Float (single-precision)"))
  (set `/Game/00_Christin/Draugr/WBP_Healthbar.HealPercent` (`KismetMathLibrary.MapRangeClamped` (`self.CurrentHealth`) 0.0 (`self.MaxHealth`) 0.0 1.0) (`self.WBPHealthbar`)))

(event `OnComponentBeginOverlap_Event`
  (params (OverlappedComponent :type "PrimitiveComponent Object Reference") (OtherActor :type "Actor Object Reference") (OtherComp :type "PrimitiveComponent Object Reference") (OtherBodyIndex :type Integer) (bFromSweep :type Boolean) (SweepResult :type "HitResult Structure (by ref)"))
  (if (and (`ActorComponent.ComponentHasTag` OtherComp "HurtZone") (`self.DamageWindow`))
    (`/Engine/EditorBlueprintResources/StandardMacros.DoOnce` false :!label _label
      (:`Completed`
        (message `/Game/00_Christin/Combat/IF_AIEnemy.CallHit` OtherActor (`self.Damage`))))))

(event `/Game/00_Christin/Combat/IF_AIEnemy.CallHit`
  (params (Hit :type "Float (double-precision)"))
  (set `self.CurrentHealth` (- (`self.CurrentHealth`) Hit))
  (if (<= (`self.CurrentHealth`) 0.0)
    (set `self.IsDead` true)
    (`self.Dying`)
    (else
      (`|PlayMontage` (`self.Mesh`) "/Game/00_Christin/Draugr/Animations/Combat/AM_Draugr_Damage.AM_Draugr_Damage" 2.0))))

(event `ResetOverlapDamageEvent`
  (goto _label :!via `Reset`))

(event `/Game/00_Christin/Combat/IF_AIEnemy.CallCombat`
  (`SceneComponent.SetHiddenInGame` (`self.HealthBar`) false false)
  (`|PlayMontage` (`self.Mesh`) "/Game/00_Christin/Draugr/Animations/Combat/AM_Draugr_Targeted.AM_Draugr_Targeted"
    (:`OnCompleted`
      _)
    (:`OnInterrupted`
      _))
  (`self.On Discovered End`))

(event `/Game/00_Christin/Combat/IF_AIEnemy.ResetHeal`
  (set `self.CurrentHealth` (`self.MaxHealth`))
  (`SceneComponent.SetHiddenInGame` (`self.HealthBar`) true false))

(event `/Game/00_Christin/Combat/IF_AIEnemy.Anim_CombatEvent`
  (bind _mesh (`self.Mesh`))
  (if (`KismetMathLibrary.RandomBool`)
    (`|PlayMontage` _mesh "/Game/00_Christin/Draugr/Animations/Combat/AM_Draugr_Attack01.AM_Draugr_Attack01" 2.0
      (:`OnCompleted`
        _)
      (:`OnInterrupted`
        _))
    (else
      (`|PlayMontage` _mesh "/Game/00_Christin/Draugr/Animations/Combat/AM_Draugr_Attack02.AM_Draugr_Attack02" 1.5
        (:`OnCompleted`
          _)
        (:`OnInterrupted`
          _))))
  (`self.On Attack End`)
  (`self.ResetOverlapDamageEvent`))

(event `/Game/00_Christin/Combat/IF_AIEnemy.CallStraggered`
  (`|PlayMontage` (`self.Mesh`) "/Game/00_Christin/Draugr/Animations/Combat/AM_Draugr_Staggerd.AM_Draugr_Staggerd" 2.0))

(event `Dying`
  (`/Engine/EditorBlueprintResources/StandardMacros.DoOnce` false
    (:`Completed`
      (`|PlayMontage` (`self.Mesh`) "/Game/00_Christin/Draugr/Animations/Combat/AM_Draugr_Dying.AM_Draugr_Dying"))))

(event `/Game/00_Christin/Combat/IF_AIEnemy.Anim_DyingEvent`
  (bind _tutorial_stack (`/Game/04_UI/Player/CAW_PlayerHUD.Tutorial_Stack` (`/Game/00_Christin/Eir/BP_Eir.CAW Player` (`/Game/00_Christin/GameMode_Eir.BPEir` (`self.GameMode`)))))
  (bind (_direction _time) (`Timeline|TL_Dying` :!via `PlayFromStart`)
    (:`Update`
      (`MeshComponent.SetScalarParameterValueOnMaterials` (`self.Mesh`) "Mask" _time))
    (:`Finished`
      (`/Game/00_Christin/Combat/BP_AreaManager.Defeated` (`self.Manager`) self)
      (if (`self.Tutorial`)
        (`CommonActivatableWidgetContainerBase.RemoveWidget` _tutorial_stack (`CommonActivatableWidgetContainerBase.GetActiveWidget` _tutorial_stack)))
      (`self.K2_DestroyActor`))))

(fn `AskDead`
  (returns (isDead :type Boolean))
  (return (`self.IsDead`)))

(fn `CallDamageWindow`
  (params (Bool :type Boolean))
  (returns (NewParam :type Boolean))
  (bind _output_get (set `self.DamageWindow` Bool))
  (return _output_get))

(fn `EnemyTyp`
  (returns (AITyp :type "/Game/00_Christin/Combat/Enumirator/E_AITyp Enum"))
  (return (`self.Typ`)))

(fn `GetIdealRange`
  (returns (AttackRadius :type "Float (double-precision)") (DefendRadius :type "Float (double-precision)"))
  (return (`self.Attack Radius`) (`self.Defend Radius`)))

(fn `MovementValue`
  (params (WalkSpeedTyp :type "/Game/00_Christin/Combat/Enumirator/E_AIWalkSpeed Enum" :default "NewEnumerator0"))
  (returns (Value :type "Float (double-precision)"))
  (bind _output_get (set `CharacterMovementComponent.MaxWalkSpeed` (select `/Game/00_Christin/Combat/Enumirator/E_AIWalkSpeed` WalkSpeedTyp :`NewEnumerator1` (`self.Patrol`) :`NewEnumerator2` (`self.Chase`)) (`self.CharacterMovement`)))
  (return _output_get))

(fn `ReturnAIEnemy`
  (params (GetAICharater :type "Pawn Object Reference"))
  (return))

(fn `UserConstructionScript`)
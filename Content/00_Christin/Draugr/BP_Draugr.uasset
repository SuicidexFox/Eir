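; BP_Draugr is a Draugr combatant that deals damage on touch and takes it only during a damage window.
; Attacking closes the window and binds overlaps on "DemegeZone"-tagged components, which send a damage message to the overlapped actor.
; Incoming damage lowers Health while the window is open; otherwise it heals, capping only when Health already reaches MaxHealth.
; Nothing here opens the window, and CallCombatStructure is an empty stub.
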(event `Attacking`
  (set `/Game/00_Christin/Combat/AC_Combat.DamageWindow` false)
  (if true
    (for _array_element (`self.GetComponentsByTag` "/Script/Engine.PrimitiveComponent" "DemegeZone")
      (add `PrimitiveComponent.OnComponentBeginOverlap` _array_element (delegate `OnComponentBeginOverlap_Event`)))))

(event `OnComponentBeginOverlap_Event`
  (params (OverlappedComponent :type "PrimitiveComponent Object Reference") (OtherActor :type "Actor Object Reference") (OtherComp :type "PrimitiveComponent Object Reference") (OtherBodyIndex :type Integer) (bFromSweep :type Boolean) (SweepResult :type "HitResult Structure (by ref)"))
  (if (`ActorComponent.ComponentHasTag` OverlappedComponent "DemegeZone")
    (message `/Game/00_Christin/Combat/IF_Combat.Damage` OtherActor (`/Game/00_Christin/Combat/AC_Combat.Damage`))))

(event `/Game/00_Christin/Combat/IF_Combat.Damage`
  (params (Damage :type "Float (double-precision)"))
  (bind _maxhealth (`/Game/00_Christin/Combat/AC_Combat.MaxHealth`))
  (bind _health (`/Game/00_Christin/Combat/AC_Combat.Health`))
  (if (`/Game/00_Christin/Combat/AC_Combat.DamageWindow`)
    (set `/Game/00_Christin/Combat/AC_Combat.Health` (- (`/Game/00_Christin/Combat/AC_Combat.Health`) Damage))
    (elif (>= _health _maxhealth)
      (set `/Game/00_Christin/Combat/AC_Combat.Health` _maxhealth)
      (else
        (set `/Game/00_Christin/Combat/AC_Combat.Health` (+ _health (`/Game/00_Christin/Combat/AC_Combat.HealAmount`)))))))

(fn `CallCombatStructure`
  (returns (CompatStructure :type "/Game/00_Christin/Combat/Structur_Combat Structure"))
  (return))

(fn `UserConstructionScript`)
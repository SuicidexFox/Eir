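; Draugr enemy character that exposes combat, movement speed and range functions, with montage-driven actions that report back when they finish.
; BeginPlay waits for GameMode_Eir, messages the AI controller and binds DamageZone overlaps, which hit HurtZone components once per attack during the ACCombat damage window.
; Incoming hits update ACCombat health and the healthbar widget.
; Dying fades the mesh through an OpacityMask timeline, notifies the combat Manager and destroys the actor.
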(event `self.ReceiveBeginPlay`
  (cast `/Game/00_Christin/GameMode_Eir` (`GameplayStatics.GetGameMode`) :!label _label
    (:`then`
      (message `/Game/00_Christin/Combat/AI_BehaviorTree/IF_AIController.ContollerBlackboard` (`AIBlueprintHelperLibrary.GetAIController` null))
      (for _array_element (`self.GetComponentsByTag` "/Script/Engine.PrimitiveComponent" "DamageZone")
        (add `PrimitiveComponent.OnComponentBeginOverlap` _array_element (`|CreateDelegate` :!event `OnComponentBeginOverlap_Event`))
        (bind _aswbp_healthbar (cast `/Game/00_Christin/Draugr/WBP_Healthbar` (`WidgetComponent.GetWidget` (`self.HealthBar`))))
        (bind _output_get (set `self.WBPHealthbar` _aswbp_healthbar))
        (set `/Game/00_Christin/Draugr/WBP_Healthbar.MaxHealth` (`/Game/00_Christin/Combat/AC_CombatValues.Health` (`self.AC_Combat`)) _output_get)))
    (:`CastFailed`
      (`KismetSystemLibrary.DelayUntilNextTick`)
      (goto _label))))

(event `/Game/00_Christin/Combat/IF_AIEnemy.AddCombatManager`
  (params (Manager :type "/Game/00_Christin/Combat/BP_AreaManager Object Reference"))
  (set `self.Manager` Manager))

(event `Idle Variance`
  (`|PlayMontage` (`self.Mesh`) (`KismetArrayLibrary.Array_Random` (`self.IdleVariance`))
    (:`OnCompleted`
      _)
    (:`OnInterrupted`
      _))
  (`self.On Idle End`))

(event `OnComponentBeginOverlap_Event`
  (params (OverlappedComponent :type "PrimitiveComponent Object Reference") (OtherActor :type "Actor Object Reference") (OtherComp :type "PrimitiveComponent Object Reference") (OtherBodyIndex :type Integer) (bFromSweep :type Boolean) (SweepResult :type "HitResult Structure (by ref)"))
  (if (and (`ActorComponent.ComponentHasTag` OtherComp "HurtZone") (`/Game/00_Christin/Combat/AC_CombatValues.DamageWindow` (`self.AC_Combat`)))
    (`/Engine/EditorBlueprintResources/StandardMacros.DoOnce` false :!label _label
      (:`Completed`
        (message `/Game/00_Christin/Combat/IF_AIEnemy.CallHit` OtherActor (`/Game/00_Christin/Combat/AC_CombatValues.Damage` (`self.AC_Combat`)))))))

(event `/Game/00_Christin/Combat/IF_AIEnemy.CallHit`
  (params (Hit :type "Float (double-precision)"))
  (bind _ac_combat (`self.AC_Combat`))
  (`/Game/00_Christin/Combat/AC_CombatValues.CallHealth` _ac_combat (- (`/Game/00_Christin/Combat/AC_CombatValues.Health` _ac_combat) Hit))
  (`/Game/00_Christin/Draugr/WBP_Healthbar.SetPercent` (`self.WBPHealthbar`) 0.0)
  (`|PlayMontage` (`self.Mesh`) "/Game/00_Christin/Draugr/Animations/Combat/AM_Draugr_Damage.AM_Draugr_Damage" 2.0
    (:`OnCompleted`
      _)
    (:`OnInterrupted`
      _))
  (`self.On Damage`))

(event `ResetOverlapDamageEvent`
  (goto _label :!via `Reset`))

(event `Discovered`
  (`|PlayMontage` (`self.Mesh`) "/Game/00_Christin/Draugr/Animations/Combat/AM_Draugr_Targeted.AM_Draugr_Targeted"
    (:`OnCompleted`
      _)
    (:`OnInterrupted`
      _))
  (`self.On Discovered End`))

(event `/Game/00_Christin/Combat/IF_AIEnemy.CallStraggered`
  (params (Hit :type "Float (double-precision)"))
  (bind _ac_combat (`self.AC_Combat`))
  (`/Game/00_Christin/Combat/AC_CombatValues.CallHealth` _ac_combat (- (`/Game/00_Christin/Combat/AC_CombatValues.Health` _ac_combat) Hit))
  (`/Game/00_Christin/Draugr/WBP_Healthbar.SetPercent` (`self.WBPHealthbar`) 0.0)
  (`|PlayMontage` (`self.Mesh`) "/Game/00_Christin/Draugr/Animations/Combat/AM_Draugr_Dying.AM_Draugr_Dying" 2.0))

(event `Attack`
  (bind _mesh (`self.Mesh`))
  (if (`KismetMathLibrary.RandomBool`)
    (`|PlayMontage` _mesh "/Game/00_Christin/Draugr/Animations/Combat/AM_Draugr_Attack01.AM_Draugr_Attack01" 2.0
      (:`OnCompleted`
        _)
      (:`OnInterrupted`
        _))
    (else
      (`|PlayMontage` _mesh "/Game/00_Christin/Draugr/Animations/Combat/AM_Draugr_Attack02.AM_Draugr_Attack02" 1.5
        (:`OnCompleted`
          _)
        (:`OnInterrupted`
          _))))
  (`self.On Attack End`)
  (`self.ResetOverlapDamageEvent`))

(event `/Game/00_Christin/Combat/IF_AIEnemy.CallDying`
  (params (Montage :type "AnimMontage Object Reference"))
  (`/Engine/EditorBlueprintResources/StandardMacros.DoOnce` false
    (:`Completed`
      (`|PlayMontage` (`self.Mesh`) Montage
        (:`then`
          (bind (_direction _time) (`Timeline|Timeline` :!via `PlayFromStart`)
            (:`Update`
              (`MeshComponent.SetScalarParameterValueOnMaterials` (`self.Mesh`) "OpacityMask" _time))))
        (:`OnCompleted`
          (`self.On Dying End` :!label _label)
          (`/Game/00_Christin/Combat/BP_AreaManager.Ready` (`self.Manager`) self)
          (`self.K2_DestroyActor`))
        (:`OnInterrupted`
          (goto _label))))))

(event `CallDeath_1_1`
  (params (NewParam1 :type Boolean))
  (bind _ac_combat (`self.AC_Combat`))
  (`ProgressBar.SetPercent` (`/Game/00_Christin/Draugr/WBP_Healthbar.HealthBar` (`self.WBPHealthbar`)) 1.0)
  (set `/Game/00_Christin/Combat/AC_CombatValues.Health` (`/Game/00_Christin/Combat/AC_CombatValues.MaxHealth` _ac_combat) _ac_combat))

(fn `CallAggro`
  (params (Bool :type Boolean))
  (return))

(fn `CallDeath`
  (bind _ac_combat (`self.AC_Combat`))
  (`ProgressBar.SetPercent` (`/Game/00_Christin/Draugr/WBP_Healthbar.HealthBar` (`self.WBPHealthbar`)) 1.0)
  (set `/Game/00_Christin/Combat/AC_CombatValues.Health` (`/Game/00_Christin/Combat/AC_CombatValues.MaxHealth` _ac_combat) _ac_combat)
  (return))

(fn `CombatValues`
  (returns (ActorComponant :type "/Game/00_Christin/Combat/AC_CombatValues Object Reference"))
  (return null))

(fn `EnemyTyp`
  (returns (AITyp :type "/Game/00_Christin/Combat/Enumirator/E_AITyp Enum"))
  (return (`self.Typ`)))

(fn `GetIdealRange`
  (returns (AttackRadius :type "Float (double-precision)") (DefendRadius :type "Float (double-precision)"))
  (return (`self.Attack Radius`) (`self.Defend Radius`)))

(fn `MovementValue`
  (params (WalkSpeedTyp :type "/Game/00_Christin/Combat/Enumirator/E_AIWalkSpeed Enum" :default "NewEnumerator0"))
  (returns (Value :type "Float (double-precision)"))
  (bind _output_get (set `CharacterMovementComponent.MaxWalkSpeed` (select `/Game/00_Christin/Combat/Enumirator/E_AIWalkSpeed` WalkSpeedTyp :`NewEnumerator0` (`self.Idle`) :`NewEnumerator1` (`self.Patrol`) :`NewEnumerator2` (`self.Chase`)) (`self.CharacterMovement`)))
  (return _output_get))

(fn `UserConstructionScript`)
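; Trigger that changes the level's directional light when any actor enters its box.
; Overlap plays the SunRotation timeline, whose Duration output blends the light's rotation and intensity toward a target on each update.
; IsFirst selects between the middle rotation with dimmer light and the end rotation with brighter light.
; Each blend starts from the light's current values rather than cached starting ones, so the change compounds over the timeline.
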(event `self.Box.OnComponentBeginOverlap`
  (params (OverlappedComponent :type "PrimitiveComponent Object Reference") (OtherActor :type "Actor Object Reference") (OtherComp :type "PrimitiveComponent Object Reference") (OtherBodyIndex :type Integer) (bFromSweep :type Boolean) (SweepResult :type "HitResult Structure (by ref)"))
  (bind _directionalight (`self.Directionalight`))
  (bind _directionalight_2 (`self.Directionalight`))
  (bind _lightcomponent (`Light.LightComponent` _directionalight))
  (bind _lightcomponent_2 (`Light.LightComponent` _directionalight_2))
  (bind (_direction _duration) (`Timeline|SunRotation`)
    (:`Update`
      (if (`self.IsFirst`)
        (`self.K2_SetActorLocationAndRotation` _directionalight_2 (0.0 0.0 0.0) (`KismetMathLibrary.RLerp` (`self.K2_GetActorRotation` (`self.Directionalight`)) (`self.RotationMittle`) _duration) true false)
        (`LightComponent.SetIntensity` _lightcomponent_2 (`KismetMathLibrary.Lerp` (`LightComponentBase.Intensity` _lightcomponent_2) 3.0 _duration))
        (else
          (`self.K2_SetActorLocationAndRotation` _directionalight (0.0 0.0 0.0) (`KismetMathLibrary.RLerp` (`self.K2_GetActorRotation` (`self.Directionalight`)) (`self.RotationEnd`) _duration) true false)
          (`LightComponent.SetIntensity` _lightcomponent (`KismetMathLibrary.Lerp` (`LightComponentBase.Intensity` _lightcomponent) 8.0 _duration)))))))

(fn `UserConstructionScript`)